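; BP_FemalePlayer is a player Blueprint that shows day-start and day-end UI in response to the game's day cycle.
; On BeginPlay it caches HDGameStateBase, binds to its status-changed event and pre-creates both widgets, giving the day-end one references to the game state and itself.
; Each status change clears both widgets, then shows the day-end widget when Idle or the day-start widget once the day has started.
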(event Custom|OnStatusChanged_Event_0
  (bind _returnvalue (Class|HDGameStateBase|GetGameStatus (Variables|Default|GetGameStateRef)))
  (switch Utilities|FlowControl|Switch|SwitchonEGameStatus _returnvalue
    (:GS_Idle
      (CallFunction|AddDayEndWidget))
    (:GS_DayStarting
      (CallFunction|RemoveGameplayWidgets))
    (:GS_DayStarted
      (CallFunction|AddDayStartWidget))
    (:GS_DayEnding
      (CallFunction|RemoveGameplayWidgets))))

(event EventBeginPlay
  (bind _ashdgame_state_base (Utilities|Casting|CastToHDGameStateBase (Game|GetGameState)))
  (bind _output_get (Variables|Default|SetGameStateRef _ashdgame_state_base))
  (EventDispatchers|AssignOnStatusChanged _output_get (delegate Custom|OnStatusChanged_Event_0))
  (bind _returnvalue (UserInterface|CreateWidget "/Game/Widgets/WBP_DayStarted.WBP_DayStarted_C" (Game|GetPlayerController 0)))
  (Variables|Default|SetDayStartWidgetRef _returnvalue)
  (bind _returnvalue_2 (UserInterface|CreateWidget "/Game/Widgets/WBP_DayEnd.WBP_DayEnd_C" (Game|GetPlayerController 0) (Variables|Default|GetGameStateRef) self))
  (Variables|Default|SetDayEndWidgetRef _returnvalue_2))

(fn ConstructionScript)

(fn RemoveGameplayWidgets
  (bind _daystartwidgetref (Variables|Default|GetDayStartWidgetRef))
  (bind _dayendwidgetref (Variables|Default|GetDayEndWidgetRef))
  (Utilities|IsValid _daystartwidgetref
    (:Is%20Valid
      (Widget|RemovefromParent _daystartwidgetref))
    (:Is%20Not%20Valid
      _))
  (Utilities|IsValid _dayendwidgetref
    (:Is%20Valid
      (Widget|RemovefromParent _dayendwidgetref))
    (:Is%20Not%20Valid
      _))
  (return))

(fn AddDayEndWidget
  (bind _dayendwidgetref (Variables|Default|GetDayEndWidgetRef))
  (CallFunction|RemoveGameplayWidgets)
  (Utilities|IsValid _dayendwidgetref
    (:Is%20Valid
      (UserInterface|Viewport|AddtoViewport _dayendwidgetref 0)
      (return))))

(fn AddDayStartWidget
  (bind _daystartwidgetref (Variables|Default|GetDayStartWidgetRef))
  (CallFunction|RemoveGameplayWidgets)
  (Utilities|IsValid _daystartwidgetref
    (:Is%20Valid
      (UserInterface|Viewport|AddtoViewport _daystartwidgetref 0)
      (return))))