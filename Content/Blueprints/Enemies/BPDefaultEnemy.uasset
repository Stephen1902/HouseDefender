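; BPDefaultEnemy is a default enemy Blueprint that keeps the enemy's health bar widget up to date when it is hit.
; On BeginPlay it binds to the OnEnemyHit event, which supplies the pawn widget and the new health.
; The first hit casts and caches the widget as WBP_EnemyHealthBar, then each hit updates its health and the colour from GetColourOfHealthBar.
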(event Custom|OnEnemyHit_Event_0
  (params (EnemyPawnWidget :type User%20Widget%20Object%20Reference) (NewEnemyHealth :type Float%20%28single-precision%29))
  (Utilities|IsValid (Variables|Default|GetAs%20Enemy%20Health%20Bar)
    (:Is%20Valid
      _)
    (:Is%20Not%20Valid
      (bind _aswbp_enemy_health_bar (Utilities|Casting|CastToWBP_EnemyHealthBar EnemyPawnWidget))
      (bind _output_get (Variables|Default|SetAs%20Enemy%20Health%20Bar _aswbp_enemy_health_bar))))
  (Default|UpdateHealth _output_get NewEnemyHealth (Class|HDEnemyMaster|GetColourOfHealthBar)))

(event EventBeginPlay
  (EventDispatchers|AssignOnEnemyHit (delegate Custom|OnEnemyHit_Event_0)))

(fn ConstructionScript)